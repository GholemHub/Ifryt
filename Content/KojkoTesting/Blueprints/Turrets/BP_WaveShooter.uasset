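; BP_WaveShooter is a turret hazard that fires projectiles from six arrow muzzles until it takes damage.
; Overlapping the start trigger begins a looping timer that picks a different random muzzle and adds another looping shoot timer without clearing earlier ones.
; The player entering the box raises the heart once.
; Any damage destroys the heart, clears the wave and latest shoot timers, and moves the platform via timeline.
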(event OnComponentBeginOverlap(Box)
  (params (OverlappedComponent :type Primitive%20Component%20Object%20Reference) (OtherActor :type Actor%20Object%20Reference) (OtherComp :type Primitive%20Component%20Object%20Reference) (OtherBodyIndex :type Integer) (bFromSweep :type Boolean) (SweepResult :type Hit%20Result%20Structure%20%28by%20ref%29))
  (if (== OtherActor (Game|GetPlayerCharacter 0))
    (Utilities|FlowControl|DoOnce false
      (:Completed
        (bind _newtrack_0 (Timeline|HeartRise Play)
          (:Update
            (Transformation|SetRelativeLocation (Variables|Default|GetHeart) (Math|Vector|MakeVector -2.3e+02 0.0 (Math|Float|Lerp 0.0 4e+02 _newtrack_0)) false false)))))))

(event OnComponentBeginOverlap(StartTrigger)
  (params (OverlappedComponent :type Primitive%20Component%20Object%20Reference) (OtherActor :type Actor%20Object%20Reference) (OtherComp :type Primitive%20Component%20Object%20Reference) (OtherBodyIndex :type Integer) (bFromSweep :type Boolean) (SweepResult :type Hit%20Result%20Structure%20%28by%20ref%29))
  (Utilities|FlowControl|DoOnce false
    (:Completed
      (bind _returnvalue (Utilities|Time|SetTimerbyEvent (delegate Custom|Wave) 1.0 true false -1.0)))))

(event Custom|Wave
  (bind _output_get (Variables|Default|SetNewGunNr (Math|Random|RandomIntegerinRange 0 5) :!label _label))
  (if (== _output_get (Variables|Default|GetGunNr))
    (goto _label)
    (else
      (Variables|Default|SetGunNr (Variables|Default|GetNewGunNr))
      (Variables|Default|SetActiveGun (Transformation|GetWorldTransform (Utilities|Select :Index (Variables|Default|GetGunNr) :Option%200 (Variables|Default|GetArrow) :Option%201 (Variables|Default|GetArrow1) :Option%202 (Variables|Default|GetArrow2) :Option%203 (Variables|Default|GetArrow3) :Option%204 (Variables|Default|GetArrow4) :Option%205 (Variables|Default|GetArrow5))))
      (bind _returnvalue (Utilities|Time|SetTimerbyEvent (delegate Custom|Shoot) 0.3 true)))))

(event Custom|Shoot
  (Game|SpawnActorfromClass "/Game/KojkoTesting/Blueprints/BP_Projectile_VFX_TempFix.BP_Projectile_VFX_TempFix_C" (Variables|Default|GetActiveGun) "Undefined" "MultiplyWithRoot" 0 0))

(event Custom|KillHeart
  (params (DamagedActor :type Actor%20Object%20Reference) (Damage :type Float%20%28single-precision%29) (DamageType :type Damage%20Type%20Object%20Reference) (InstigatedBy :type Controller%20Object%20Reference) (DamageCauser :type Actor%20Object%20Reference))
  (Utilities|Time|ClearandInvalidateTimerbyHandle (stale OnComponentBeginOverlap(StartTrigger) _returnvalue))
  (Utilities|Time|ClearandInvalidateTimerbyHandle (stale Custom|Wave _returnvalue))
  (Components|DestroyComponent (Variables|Default|GetHeart))
  (bind _newtrack_0 (Timeline|PlatformRise Play)
    (:Update
      (Transformation|SetRelativeLocation (Variables|Default|GetPlatform) (Math|Vector|MakeVector 909.0 0.0 (Math|Float|Lerp (.z (Variables|/Script/Engine.SceneComponent|GetRelativeLocation (Variables|Default|GetPlatform))) -3e+02 _newtrack_0)) false false))))

(event EventBeginPlay
  (EventDispatchers|AssignOnTakeAnyDamage (delegate Custom|KillHeart)))

(fn ConstructionScript)