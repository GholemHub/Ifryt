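; Turret that calls timed thunder strikes on random nearby points or the player's position.
; A one-time looping timer, started by player trigger overlap or Phase2 during a boss fight, runs Aim while the player is within TargetRadius.
; Aim spawns the Niagara effect and stores AimPosition, re-rolling random picks for each, then a delayed Shoot sphere-traces there and applies damage.
; The construction script draws TargetRadius as a debug sphere.
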(event OnComponentBeginOverlap(StartTrigger)
  (params (OverlappedComponent :type Primitive%20Component%20Object%20Reference) (OtherActor :type Actor%20Object%20Reference) (OtherComp :type Primitive%20Component%20Object%20Reference) (OtherBodyIndex :type Integer) (bFromSweep :type Boolean) (SweepResult :type Hit%20Result%20Structure%20%28by%20ref%29))
  (if (== OtherActor (Game|GetPlayerCharacter 0))
    (Utilities|FlowControl|DoOnce false
      (:Completed
        (Utilities|Time|SetTimerbyEvent (delegate Custom|Aim) 3.0 true false 0.0 1.5)))))

(event Custom|Aim
  (bind _returnvalue (Transformation|GetActorLocation))
  (bind _returnvalue_2 (Math|Random|RandomUnitVector))
  (bind _returnvalue_3 (Math|Random|RandomFloatinRange 3e+02 6.8e+03))
  (bind _returnvalue_4 (Game|GetPlayerCharacter 0))
  (bind _random (Variables|Default|GetRandom))
  (bind _returnvalue_5 (Transformation|GetActorLocation _returnvalue_4))
  (bind _returnvalue_6 (* _returnvalue_2 _returnvalue_3))
  (bind _returnvalue_7 (+ _returnvalue _returnvalue_6))
  (bind _returnvalue_8 (Math|Vector|SelectVector _returnvalue_7 _returnvalue_5 _random))
  (bind (_x _y) (Math|Vector|BreakVector _returnvalue_8))
  (if (<= (Math|Vector|Distance(Vector) _returnvalue _returnvalue_5) (Variables|Default|GetTargetRadius))
    (Niagara|SpawnSystematLocation "/Game/_Characters/NPC/NPC_VFX/Thunder/NS_ThunderStrike.NS_ThunderStrike" (Math|Vector|MakeVector _x _y 1.48e+03))
    (Variables|Default|SetAimPosition (Math|Vector|MakeVector _x _y 1.48e+03))
    (Utilities|Time|SetTimerbyEvent (delegate Custom|Shoot) 2.0)))

(event Custom|Shoot
  (bind _aimposition (Variables|Default|GetAimPosition))
  (bind _outhits (Collision|MultiSphereTraceByChannel _aimposition _aimposition 2e+02 "TraceTypeQuery1" false 0 "None" true "(R=0.000000,G=0.136006,B=1.000000,A=1.000000)" "(R=0.000000,G=1.000000,B=0.000000,A=1.000000)" 1.0))
  (for _array_element _outhits
    (Game|Damage|ApplyDamage (.HitActor (Collision|BreakHitResult _array_element)) 5e+01 0 0 "/Game/KojkoTesting/Blueprints/BP_TurretDamageClass.BP_TurretDamageClass_C")))

(event EventPhase2
  (if (Variables|Default|GetBossFight)
    (Utilities|FlowControl|DoOnce false
      (:Completed
        (Utilities|Time|SetTimerbyEvent (delegate Custom|Aim) 3.0 true false 0.0 1.5)))))

(fn ConstructionScript
  (Rendering|Debug|DrawDebugSphere (Transformation|GetActorLocation) (Variables|Default|GetTargetRadius) 12 "(R=1.000000,G=1.000000,B=1.000000,A=1.000000)" 0.0 5.0))