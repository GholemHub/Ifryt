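; A test cube actor that both takes and deals damage, showing its remaining health on a text element.
; BeginPlay fills health from a max value and binds to its own any-damage event, which subtracts damage, updates the text and destroys the actor at zero or below.
; Hitting another actor applies fixed damage to it, throttled by a DoOnce that resets after a short delay.
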(event Custom|OnTakeAnyDamage_Event
  (params (DamagedActor :type Actor%20Object%20Reference) (Damage :type Float%20%28single-precision%29) (DamageType :type Damage%20Type%20Object%20Reference) (InstigatedBy :type Controller%20Object%20Reference) (DamageCauser :type Actor%20Object%20Reference))
  (Variables|Default|SetCubeHP (- (Variables|Default|GetCubeHP) Damage))
  (Rendering|Components|TextRender|SetText (Variables|Default|GetHPtext) (Utilities|Text|ToText(Integer) (Variables|Default|GetCubeHP)))
  (if (<= (Variables|Default|GetCubeHP) 0)
    (Actor|DestroyActor)))

(event EventBeginPlay
  (bind _cubemaxhp (Variables|Default|GetCubeMaxHp))
  (EventDispatchers|AssignOnTakeAnyDamage (delegate Custom|OnTakeAnyDamage_Event))
  (Rendering|Components|TextRender|SetText (Variables|Default|GetHPtext) (Utilities|Text|ToText(Integer) _cubemaxhp))
  (Variables|Default|SetCubeHP _cubemaxhp))

(event EventTick
  (params (DeltaSeconds :type Float%20%28single-precision%29)))

(event Collision|EventHit
  (params (MyComp :type Primitive%20Component%20Object%20Reference) (Other :type Actor%20Object%20Reference) (OtherComp :type Primitive%20Component%20Object%20Reference) (bSelfMoved :type Boolean) (HitLocation :type Vector :default "0, 0, 0") (HitNormal :type Vector :default "0, 0, 0") (NormalImpulse :type Vector :default "0, 0, 0") (Hit :type Hit%20Result%20Structure%20%28by%20ref%29))
  (Utilities|FlowControl|DoOnce false :!label _label
    (:Completed
      (Game|Damage|ApplyDamage Other 1e+01 0 0)
      (Utilities|FlowControl|Delay 0.5)
      (goto _label Reset))))

(fn ConstructionScript)