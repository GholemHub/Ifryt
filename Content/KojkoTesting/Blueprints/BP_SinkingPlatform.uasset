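; Sinking platform actor that appears as a random small rock and moves vertically when hit.
; On BeginPlay it picks one of four rock meshes for the Platform component.
; A hit on the Platform plays a timeline that lerps its relative Z between zero and the Height variable's Z.
; A DoOnce gate ignores further hits until the timeline finishes.
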(event OnComponentHit(Platform)
  (params (HitComponent :type Primitive%20Component%20Object%20Reference) (OtherActor :type Actor%20Object%20Reference) (OtherComp :type Primitive%20Component%20Object%20Reference) (NormalImpulse :type Vector :default "0, 0, 0") (Hit :type Hit%20Result%20Structure%20%28by%20ref%29))
  (Utilities|FlowControl|DoOnce false :!label _label
    (:Completed
      (bind _newtrack_0 (Timeline|SinkTimeline PlayFromStart)
        (:Update
          (Transformation|SetRelativeLocation (Variables|Default|GetPlatform) (Math|Vector|MakeVector 0.0 0.0 (Math|Float|Lerp 0.0 (.z (Variables|Default|GetHeight)) _newtrack_0)) false false))
        (:Finished
          (goto _label Reset))))))

(event EventBeginPlay
  (Components|StaticMesh|SetStaticMesh (Variables|Default|GetPlatform) (Utilities|Select :Index (Math|Random|RandomIntegerinRange 0 3) :Option%200 "/Game/_Enviro_Assets/Rocks/Meshes/Small_Rock_01.Small_Rock_01" :Option%201 "/Game/_Enviro_Assets/Rocks/Meshes/Small_Rock_02.Small_Rock_02" :Option%202 "/Game/_Enviro_Assets/Rocks/Meshes/Small_Rock_03.Small_Rock_03" :Option%203 "/Game/_Enviro_Assets/Rocks/Meshes/Small_Rock_04.Small_Rock_04")))

(event Collision|EventActorBeginOverlap
  (params (OtherActor :type Actor%20Object%20Reference)))

(event EventTick
  (params (DeltaSeconds :type Float%20%28single-precision%29)))

(fn ConstructionScript)