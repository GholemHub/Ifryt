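; Boss actor for a five-phase fight, started by a trigger that closes tagged doors and signals turrets.
; Player damage depletes HP, advancing phases through targeted shots, rotating lasers, four-way fire, a barrier-backed enemy wave, then hard-mode lasers.
; Looping timers drive rotation, firing and beam-end traces, while overlap volumes deal laser damage.
; An expanding capsule-trace shockwave exists but is never triggered here, and final-phase defeat does nothing.
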(event OnComponentBeginOverlap(LaserLow)
  (params (OverlappedComponent :type Primitive%20Component%20Object%20Reference) (OtherActor :type Actor%20Object%20Reference) (OtherComp :type Primitive%20Component%20Object%20Reference) (OtherBodyIndex :type Integer) (bFromSweep :type Boolean) (SweepResult :type Hit%20Result%20Structure%20%28by%20ref%29))
  ;[0.1392 0.9792 0 0.5] Lasers
  (if (Variables|Default|GetLaserActiveLow)
    (if (== OtherActor (Game|GetPlayerCharacter 0))
      (Variables|Default|SetLaserHit OtherActor)
      (Utilities|FlowControl|DoOnce false :!label _label
        (:Completed
          (Game|Damage|ApplyDamage (Variables|Default|GetLaserHit) 25.0 0 0)
          (Utilities|FlowControl|Delay 0.5)
          (goto _label Reset))))))

(event OnComponentBeginOverlap(StartTrigger)
  (params (OverlappedComponent :type Primitive%20Component%20Object%20Reference) (OtherActor :type Actor%20Object%20Reference) (OtherComp :type Primitive%20Component%20Object%20Reference) (OtherBodyIndex :type Integer) (bFromSweep :type Boolean) (SweepResult :type Hit%20Result%20Structure%20%28by%20ref%29))
  ;[0.15 0.15 0.15 0.5] Start fight
  (Utilities|FlowControl|DoOnce false
    (:Completed
      (EventDispatchers|BindEventtoOnTakeAnyDamage (delegate Custom|TakeDamage))
      (Variables|Default|SetBossFightStarted? true)
      (CallFunction|StartTargetedShooting)
      (bind _outactors (Actor|GetAllActorsOfClass "/Game/KojkoTesting/Blueprints/Turrets/BP_Turret.BP_Turret_C"))
      (Class|BPIBossFight|Phase2(Message) _outactors)
      (bind _outactors_2 (Actor|GetAllActorsOfClass "/Game/_AI/BP_Door.BP_Door_C"))
      (for _array_element _outactors_2
        (if (== (Variables|/Game/_AI/BP_Door.BP_Door_C|GetTag _array_element) 7)
          (Default|OnCloseEvent _array_element))))))

(event OnComponentBeginOverlap(LaserMedium)
  (params (OverlappedComponent :type Primitive%20Component%20Object%20Reference) (OtherActor :type Actor%20Object%20Reference) (OtherComp :type Primitive%20Component%20Object%20Reference) (OtherBodyIndex :type Integer) (bFromSweep :type Boolean) (SweepResult :type Hit%20Result%20Structure%20%28by%20ref%29))
  ;[0.1392 0.9792 0 0.5] Lasers
  (if (Variables|Default|GetLaserActiveMedium)
    (if (== OtherActor (Game|GetPlayerCharacter 0))
      (Variables|Default|SetLaserHit OtherActor)
      (Utilities|FlowControl|DoOnce false :!label _label
        (:Completed
          (Game|Damage|ApplyDamage (Variables|Default|GetLaserHit) 25.0 0 0)
          (Utilities|FlowControl|Delay 0.5)
          (goto _label Reset))))))

(event OnComponentBeginOverlap(LaserHigh)
  (params (OverlappedComponent :type Primitive%20Component%20Object%20Reference) (OtherActor :type Actor%20Object%20Reference) (OtherComp :type Primitive%20Component%20Object%20Reference) (OtherBodyIndex :type Integer) (bFromSweep :type Boolean) (SweepResult :type Hit%20Result%20Structure%20%28by%20ref%29))
  ;[0.1392 0.9792 0 0.5] Lasers
  (if (Variables|Default|GetLaserActiveHigh)
    (if (== OtherActor (Game|GetPlayerCharacter 0))
      (Variables|Default|SetLaserHit OtherActor)
      (Utilities|FlowControl|DoOnce false :!label _label
        (:Completed
          (Game|Damage|ApplyDamage (Variables|Default|GetLaserHit) 25.0 0 0)
          (Utilities|FlowControl|Delay 0.5)
          (goto _label Reset))))))

(event OnComponentBeginOverlap(LaserVeryHigh)
  (params (OverlappedComponent :type Primitive%20Component%20Object%20Reference) (OtherActor :type Actor%20Object%20Reference) (OtherComp :type Primitive%20Component%20Object%20Reference) (OtherBodyIndex :type Integer) (bFromSweep :type Boolean) (SweepResult :type Hit%20Result%20Structure%20%28by%20ref%29))
  ;[0.1392 0.9792 0 0.5] Lasers
  (if (Variables|Default|GetLaserActiveVeryHigh)
    (if (== OtherActor (Game|GetPlayerCharacter 0))
      (Variables|Default|SetLaserHit OtherActor)
      (Utilities|FlowControl|DoOnce false :!label _label
        (:Completed
          (Game|Damage|ApplyDamage (Variables|Default|GetLaserHit) 25.0 0 0)
          (Utilities|FlowControl|Delay 0.5)
          (goto _label Reset))))))

(event Custom|TakeDamage
  (params (DamagedActor :type Actor%20Object%20Reference) (Damage :type Float%20%28single-precision%29) (DamageType :type Damage%20Type%20Object%20Reference) (InstigatedBy :type Controller%20Object%20Reference) (DamageCauser :type Actor%20Object%20Reference))
  ;[0.15 0.15 0.15 0.5] Take Damage / Trigger Phases
  (if (== DamageCauser (Game|GetPlayerCharacter 0))
    (if (> (- (Variables|Default|GetHP) Damage) 0.0)
      (bind _output_get (Variables|Default|SetHP (- (Variables|Default|GetHP) Damage)))
      (else
        (Variables|Default|SetHP 0.0)))
    (Rendering|Components|TextRender|SetText (Variables|Default|GetHpDebug) (Utilities|Text|ToText(Float) _output_get "HalfToEven"))
    (if (<= (Variables|Default|GetHP) 0.0)
      (if (== (Variables|Default|GetPhase) 1)
        (Utilities|FlowControl|DoOnce false
          (:Completed
            (CallFunction|Phase2)))
        (elif (== (Variables|Default|GetPhase) 2)
          (Utilities|FlowControl|DoOnce false
            (:Completed
              (CallFunction|Phase3)))
          (elif (== (Variables|Default|GetPhase) 3)
            (Utilities|FlowControl|DoOnce false
              (:Completed
                (CallFunction|Phase4)))
            (elif (== (Variables|Default|GetPhase) 4)
              (Utilities|FlowControl|DoOnce false
                (:Completed
                  (CallFunction|Phase5)))
              (elif (== (Variables|Default|GetPhase) 5)
                (Utilities|FlowControl|DoOnce false)))))))))

(event Custom|StartShooting
  (bind _cooldown (Variables|Default|GetCooldown))
  ;[0.15 0.15 0.15 0.5] Shooting
  (bind _returnvalue (Utilities|Time|SetTimerbyEvent (delegate Custom|Fire) _cooldown true false (* _cooldown -1.0)))
  (Variables|Default|SetShootimgTimer _returnvalue)
  (CallFunction|StartRotating))

(event Custom|Shockwave
  (bind _returnvalue (Transformation|GetActorLocation))
  (bind _returnvalue_2 (- (.z _returnvalue) 7e+02))
  (bind _returnvalue_3 (Math|Vector|MakeVector (.x _returnvalue) (.y _returnvalue) _returnvalue_2))
  ;[1 0.5968 0.002049 0.5] Shockwave
  (if (<= (Variables|Default|GetShockwaveExpand) 5e+03)
    (bind _output_get (Variables|Default|SetShockwaveExpand (+ (Variables|Default|GetShockwaveExpand) 2e+01)))
    (Transformation|SetWorldScale3D (Variables|Default|GetShockwaveNS) (Math|Vector|MakeVector (Math|Float|Lerp 1.0 125.0 (/ _output_get 5e+03)) (Math|Float|Lerp 1.0 125.0 (/ _output_get 5e+03)) 1.0))
    (bind _outhits (Class|KismetSystemLibrary|CapsuleTraceMulti _returnvalue_3 _returnvalue_3 _output_get 1.0 "TraceTypeQuery1" false 0 "None" true))
    (for _array_element _outhits
      (if (== (.HitActor (Collision|BreakHitResult _array_element)) (Game|GetPlayerCharacter 0))
        (Utilities|FlowControl|DoOnce false
          (:Completed
            (if (not (> (.Z (Math|Vector|BreakVector (.ImpactPoint (Collision|BreakHitResult _array_element)))) 1.55e+03))
              (Game|Damage|ApplyDamage (.HitActor (Collision|BreakHitResult _array_element)) 5e+01 0 0)
              (Development|PrintString (Utilities|String|ToString(Float) (.Z (Math|Vector|BreakVector (.ImpactPoint (Collision|BreakHitResult _array_element)))))))))))
    (else
      (Utilities|Time|ClearandInvalidateTimerbyHandle (stale Custom|StartShockwave _returnvalue))
      (Variables|Default|SetShockwaveExpand 0.0))))

(event Custom|StartTargetedShooting
  ;[0.15 0 0.000759 0.5] TargetedShooting
  (bind _returnvalue (Utilities|Time|SetTimerbyEvent (delegate Custom|TargetedShooting) (Variables|Default|GetTargetedCooldowm) true))
  (Variables|Default|SetTargetedTimer _returnvalue))

(event Custom|TargetedShooting
  (bind _arrow8_targetedshooting_ (Variables|Default|GetArrow8%28targetedShooting%29))
  (bind _returnvalue (Transformation|GetWorldLocation _arrow8_targetedshooting_))
  ;[0.15 0 0.000759 0.5] TargetedShooting
  (Game|SpawnActorfromClass "/Game/KojkoTesting/Blueprints/BP_Projectile_VFX_TempFix.BP_Projectile_VFX_TempFix_C" (Math|Transform|MakeTransform _returnvalue (Math|Rotator|FindLookatRotation _returnvalue (Transformation|GetActorLocation (Game|GetPlayerCharacter 0))) "1.000000,1.000000,1.000000") "Undefined" "MultiplyWithRoot" 0 0))

(event Custom|EndRotation
  ;[0.15 0.15 0.15 0.5] End Rotation
  (Utilities|Time|ClearandInvalidateTimerbyHandle (Variables|Default|GetRotateTimer))
  (bind _returnvalue (Utilities|Time|SetTimerbyEvent (delegate Custom|RotateToStart) 0.01 true)))

(event Custom|EndLasers
  ;[0.1392 0.9792 0 0.5] Lasers
  (Variables|Default|SetLaserActiveLow false)
  (Variables|Default|SetLaserActiveMedium false)
  (Variables|Default|SetLaserActiveHigh false)
  (Variables|Default|SetLaserActiveVeryHigh false)
  (CallFunction|SetLaserVisibility))

(event Custom|LaserActivate
  (bind _n1 (Variables|Default|GetN1))
  (bind _n2 (Variables|Default|GetN2))
  (bind _n4 (Variables|Default|GetN4))
  (bind _n3 (Variables|Default|GetN3))
  (bind _returnvalue (Transformation|GetWorldLocation _n4))
  (bind _returnvalue_2 (Transformation|GetWorldLocation _n1))
  (bind _returnvalue_3 (Transformation|GetWorldLocation _n2))
  (bind _returnvalue_4 (Transformation|GetWorldLocation _n3))
  ;[0.1392 0.9792 0 0.5] Lasers
  (Utilities|FlowControl|Sequence
    (:then_0
      (if (Variables|Default|GetLaserActiveLow)
        (bind _outhit (Collision|LineTraceByChannel _returnvalue_2 (+ _returnvalue_2 (* (Math|Vector|GetForwardVector _n1) 1e+04)) "TraceTypeQuery1" false 0 "None"))
        (Class|NiagaraComponent|SetNiagaraVariableVec3 (Variables|Default|GetNiagara) "Beam End" (Math|Vector|SelectVector (.ImpactNormal (Collision|BreakHitResult _outhit)) (.TraceEnd (Collision|BreakHitResult _outhit)) false))))
    (:then_1
      (if (Variables|Default|GetLaserActiveMedium)
        (bind _outhit_2 (Collision|LineTraceByChannel _returnvalue_3 (+ _returnvalue_3 (* (Math|Vector|GetForwardVector _n2) 1e+04)) "TraceTypeQuery1" false 0 "None"))
        (Class|NiagaraComponent|SetNiagaraVariableVec3 (Variables|Default|GetNiagara1) "Beam End" (Math|Vector|SelectVector (.ImpactNormal (Collision|BreakHitResult _outhit_2)) (.TraceEnd (Collision|BreakHitResult _outhit_2)) false))))
    (:then_2
      (if (Variables|Default|GetLaserActiveHigh)
        (bind _outhit_3 (Collision|LineTraceByChannel _returnvalue_4 (+ _returnvalue_4 (* (Math|Vector|GetForwardVector _n3) 1e+04)) "TraceTypeQuery1" false 0 "None"))
        (Class|NiagaraComponent|SetNiagaraVariableVec3 (Variables|Default|GetNiagara2) "Beam End" (Math|Vector|SelectVector (.ImpactNormal (Collision|BreakHitResult _outhit_3)) (.TraceEnd (Collision|BreakHitResult _outhit_3)) false))))
    (:then_3
      (if (Variables|Default|GetLaserActiveVeryHigh)
        (bind _outhit_4 (Collision|LineTraceByChannel _returnvalue (+ _returnvalue (* (Math|Vector|GetForwardVector _n4) 1e+04)) "TraceTypeQuery1" false 0 "None"))
        (Class|NiagaraComponent|SetNiagaraVariableVec3 (Variables|Default|GetNiagara3) "Beam End" (Math|Vector|SelectVector (.ImpactNormal (Collision|BreakHitResult _outhit_4)) (.TraceEnd (Collision|BreakHitResult _outhit_4)) false))))))

(event Custom|MultiShockwave
  ;[1 0.5968 0.002049 0.5] Shockwave
  (bind _returnvalue (Utilities|Time|SetTimerbyEvent (delegate Custom|StartShockwave) 3.0 true))
  (Variables|Default|SetShockwaveTimer _returnvalue))

(event Custom|Fire
  ;[0.15 0.15 0.15 0.5] Shooting
  (for _index (range 0 3)
    (Game|SpawnActorfromClass "/Game/KojkoTesting/Blueprints/BP_Projectile_VFX_Boss.BP_Projectile_VFX_Boss_C" (Transformation|GetWorldTransform (Utilities|Select :Index _index :Option%200 (Variables|Default|GetArrow) :Option%201 (Variables|Default|GetArrow1) :Option%202 (Variables|Default|GetArrow2) :Option%203 (Variables|Default|GetArrow3))) "Undefined" "MultiplyWithRoot" 0 0)))

(event Custom|Rotate
  ;[0.15 0.15 0.15 0.5] Rotation
  (bind _output_get (Variables|Default|SetRotation (+ (Variables|Default|GetRotation) 1.0)))
  (Transformation|SetActorRotation (Math|Rotator|MakeRotator 0.0 0.0 _output_get)))

(event Custom|RotateToStart
  (bind _returnvalue (Transformation|GetActorRotation))
  ;[0.15 0.15 0.15 0.5] End Rotation
  (bind _output_get (Variables|Default|SetRotation (+ (Variables|Default|GetRotation) (select (<= (.yaw _returnvalue) 9e+01) 1.0 -1.0))))
  (Transformation|SetActorRotation (Math|Rotator|MakeRotator 0.0 0.0 _output_get))
  (if (== (.yaw _returnvalue) 9e+01)
    (Utilities|Time|ClearandInvalidateTimerbyHandle (stale Custom|EndRotation _returnvalue))))

(event Custom|EnemiesCleared
  (bind _returnvalue (Actor|GetActorOfClass "/Game/KojkoTesting/Blueprints/BP_Barrier.BP_Barrier_C"))
  (Actor|DestroyActor _returnvalue))

(event Custom|StartRotating
  ;[0.15 0.15 0.15 0.5] Rotation
  (bind _returnvalue (Utilities|Time|SetTimerbyEvent (delegate Custom|Rotate) 0.01 true))
  (Variables|Default|SetRotateTimer _returnvalue))

(event Custom|SetLasers
  ;[0.1392 0.9792 0 0.5] Lasers
  ;;[0.15 0.15 0.15 0.5] Selecting Lasers
  (bind _output_get (Variables|Default|SetNewLaserSetup (Math|Random|RandomIntegerinRange 0 2) :!label _label))
  (if (== _output_get (Variables|Default|GetLaserSetup))
    (goto _label)
    (else
      (bind _output_get_2 (Variables|Default|SetLaserSetup (Variables|Default|GetNewLaserSetup)))
      (if (Variables|Default|GetHardMode)
        (switch int _output_get_2
          (:0
            (Variables|Default|SetLaserActiveLow false)
            (Variables|Default|SetLaserActiveMedium true)
            (Variables|Default|SetLaserActiveHigh true)
            (Variables|Default|SetLaserActiveVeryHigh true))
          (:1
            (Variables|Default|SetLaserActiveLow true)
            (Variables|Default|SetLaserActiveMedium true)
            (Variables|Default|SetLaserActiveHigh true)
            (Variables|Default|SetLaserActiveVeryHigh false))
          (:2
            (Variables|Default|SetLaserActiveLow false)
            (Variables|Default|SetLaserActiveMedium true)
            (Variables|Default|SetLaserActiveHigh true)
            (Variables|Default|SetLaserActiveVeryHigh true)))
        (else
          (switch int _output_get_2
            (:0
              (Variables|Default|SetLaserActiveLow true)
              (Variables|Default|SetLaserActiveMedium false)
              (Variables|Default|SetLaserActiveHigh false)
              (Variables|Default|SetLaserActiveVeryHigh true))
            (:1
              (Variables|Default|SetLaserActiveLow false)
              (Variables|Default|SetLaserActiveMedium true)
              (Variables|Default|SetLaserActiveHigh true)
              (Variables|Default|SetLaserActiveVeryHigh false))
            (:2
              (Variables|Default|SetLaserActiveLow true)
              (Variables|Default|SetLaserActiveMedium true)
              (Variables|Default|SetLaserActiveHigh false)
              (Variables|Default|SetLaserActiveVeryHigh false)))))
      (CallFunction|SetLaserVisibility)
      (Utilities|Time|SetTimerbyEvent (delegate Custom|LaserActivate) 0.01 true))))

(event Custom|StartShockwave
  ;[1 0.5968 0.002049 0.5] Shockwave
  (bind _returnvalue (Utilities|Time|SetTimerbyEvent (delegate Custom|Shockwave) 0.01 true))
  (Utilities|FlowControl|DoOnce false) ; enters at Reset
)

(event EventPhase3
  ;[0.15 0.15 0.15 0.5] Phase 3
  (CallFunction|EndLasers)
  (Utilities|Time|ClearandInvalidateTimerbyHandle (Variables|Default|GetRotateTimer))
  (Utilities|Time|ClearandInvalidateTimerbyHandle (Variables|Default|GetTargetedTimer))
  (CallFunction|StartRotating)
  (CallFunction|StartShooting)
  (bind _output_get (Variables|Default|SetHP 1e+03))
  (Rendering|Components|TextRender|SetText (Variables|Default|GetHpDebug) (Utilities|Text|ToText(Float) _output_get "HalfToEven"))
  (bind _output_get_2 (Variables|Default|SetPhase 3))
  (Rendering|Components|TextRender|SetText (Variables|Default|GetPhaseDebug) (Utilities|Text|ToText(Integer) _output_get_2)))

(event EventPhase4
  ;[0.15 0.15 0.15 0.5] Phase 4 (add enemies spawn)
  (Utilities|Time|ClearandInvalidateTimerbyHandle (Variables|Default|GetShootimgTimer))
  (Utilities|Time|ClearandInvalidateTimerbyHandle (Variables|Default|GetRotateTimer))
  (CallFunction|EndRotation)
  (bind _returnvalue (Actor|GetActorOfClass "/Game/KojkoTesting/Blueprints/BP_Barrier.BP_Barrier_C"))
  (Class|BPIBossFight|Phase4(Message) _returnvalue)
  (Utilities|FlowControl|Delay 1.0)
  (bind _output_get (Variables|Default|SetHP 1e+03))
  (Rendering|Components|TextRender|SetText (Variables|Default|GetHpDebug) (Utilities|Text|ToText(Float) _output_get "HalfToEven"))
  (bind _output_get_2 (Variables|Default|SetPhase 4))
  (Rendering|Components|TextRender|SetText (Variables|Default|GetPhaseDebug) (Utilities|Text|ToText(Integer) _output_get_2))
  (bind _returnvalue_2 (Actor|GetActorOfClass "/Game/_AI/AI_New/CombatManager/BP_WaweManager_alter_Boss.BP_WaweManager_alter_Boss_C"))
  (Utilities|IsValid _returnvalue_2
    (:Is%20Valid
      (Default|OnStart _returnvalue_2)
      (bind _outactors (Actor|GetAllActorsOfClass "/Game/KojkoTesting/Blueprints/Turrets/BP_Turret.BP_Turret_C"))
      (for _array_element _outactors
        (Default|Stop _array_element))
      (Utilities|Time|ClearandInvalidateTimerbyHandle (Variables|Default|GetShockwaveTimer)))))

(event EventPhase5
  ;[0.15 0.15 0.15 0.5] Phase 5
  (Variables|Default|SetHardMode true)
  (CallFunction|StartRotating)
  (CallFunction|SetLasers)
  (Utilities|Time|ClearandInvalidateTimerbyHandle (Variables|Default|GetShockwaveTimer))
  (CallFunction|StartTargetedShooting)
  (bind _output_get (Variables|Default|SetHP 1e+03))
  (Rendering|Components|TextRender|SetText (Variables|Default|GetHpDebug) (Utilities|Text|ToText(Float) _output_get "HalfToEven"))
  (bind _output_get_2 (Variables|Default|SetPhase 5))
  (Rendering|Components|TextRender|SetText (Variables|Default|GetPhaseDebug) (Utilities|Text|ToText(Integer) _output_get_2)))

(event EventPhase2
  ;[0.15 0.15 0.15 0.5] Phase 2
  (CallFunction|StartRotating)
  (CallFunction|SetLasers)
  (bind _outactors (Actor|GetAllActorsOfClass "/Game/KojkoTesting/Blueprints/Turrets/BP_Turret.BP_Turret_C"))
  (Class|BPIBossFight|Phase2(Message) _outactors)
  (Variables|Default|SetTargetedCooldowm 0.5)
  (Utilities|Time|ClearandInvalidateTimerbyHandle (Variables|Default|GetTargetedTimer))
  (CallFunction|StartTargetedShooting)
  (bind _output_get (Variables|Default|SetHP 1e+03))
  (Rendering|Components|TextRender|SetText (Variables|Default|GetHpDebug) (Utilities|Text|ToText(Float) _output_get "HalfToEven"))
  (bind _output_get_2 (Variables|Default|SetPhase 2))
  (Rendering|Components|TextRender|SetText (Variables|Default|GetPhaseDebug) (Utilities|Text|ToText(Integer) _output_get_2)))

(fn ConstructionScript)

(fn SetLaserVisibility
  (Rendering|SetVisibility (Variables|Default|GetNiagara) (Variables|Default|GetLaserActiveLow) false)
  (Rendering|SetVisibility (Variables|Default|GetNiagara1) (Variables|Default|GetLaserActiveMedium) false)
  (Rendering|SetVisibility (Variables|Default|GetNiagara2) (Variables|Default|GetLaserActiveHigh) false)
  (Rendering|SetVisibility (Variables|Default|GetNiagara3) (Variables|Default|GetLaserActiveVeryHigh) false)
  (return))