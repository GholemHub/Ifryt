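; BP_BossWeakpoint is a weakpoint actor for the boss fight that responds only to turret damage.
; It binds to its own any-damage event and, on the first hit of the turret damage class, switches to a danger material and calls WeakpointTriggerMessage on the BP_Boss found in the level.
; A Phase2 event sets the Weakpoint component to a new relative position.
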(event Custom|TakeDamage
  (params (DamagedActor :type Actor%20Object%20Reference) (Damage :type Float%20%28single-precision%29) (DamageType :type Damage%20Type%20Object%20Reference) (InstigatedBy :type Controller%20Object%20Reference) (DamageCauser :type Actor%20Object%20Reference))
  (if (== (Utilities|GetClass DamageType) "/Game/KojkoTesting/Blueprints/BP_TurretDamageClass.BP_TurretDamageClass_C")
    (Utilities|FlowControl|DoOnce false
      (:Completed
        (Rendering|Material|SetMaterial (Variables|Default|GetWeakpoint) 0 "/Game/KojkoTesting/Materials/M_Danger.M_Danger")
        (bind _returnvalue (Actor|GetActorOfClass "/Game/KojkoTesting/Blueprints/Boss/BP_Boss.BP_Boss_C"))
        (Class|BPIBossFight|WeakpointTrigger(Message) _returnvalue)))))

(event EventBeginPlay
  (EventDispatchers|BindEventtoOnTakeAnyDamage (delegate Custom|TakeDamage)))

(event EventPhase2
  (Transformation|SetRelativeLocation (Variables|Default|GetWeakpoint) "0.000000,0.000000,50.000000" false false))

(fn ConstructionScript)