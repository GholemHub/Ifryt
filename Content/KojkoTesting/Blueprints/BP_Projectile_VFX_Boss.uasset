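; Boss projectile actor that damages the player on hit, with its static mesh hidden at BeginPlay.
; A hit on the first player character applies fixed damage, and a hit on anything destroys the projectile.
; A short timer started at BeginPlay also destroys it, capping its lifetime.
; A separate Destroy function wraps DestroyActor.
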(event Custom|CustomEvent
  (Actor|DestroyActor))

(event EventBeginPlay
  (Development|SetHiddeninGame (Variables|Default|GetStaticMesh) true false)
  (Utilities|Time|SetTimerbyEvent (delegate Custom|CustomEvent) 2.5))

(event EventTick
  (params (DeltaSeconds :type Float%20%28single-precision%29)))

(event Collision|EventHit
  (params (MyComp :type Primitive%20Component%20Object%20Reference) (Other :type Actor%20Object%20Reference) (OtherComp :type Primitive%20Component%20Object%20Reference) (bSelfMoved :type Boolean) (HitLocation :type Vector :default "0, 0, 0") (HitNormal :type Vector :default "0, 0, 0") (NormalImpulse :type Vector :default "0, 0, 0") (Hit :type Hit%20Result%20Structure%20%28by%20ref%29))
  (if (== Other (Game|GetPlayerCharacter 0))
    (Game|Damage|ApplyDamage Other 25.0 0 0))
  (Actor|DestroyActor))

(fn ConstructionScript)

(fn Destroy
  (Actor|DestroyActor))