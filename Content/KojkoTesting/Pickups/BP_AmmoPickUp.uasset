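; BP_AmmoPickUp is a pickup that fully refills the player's shotgun ammo.
; On actor overlap with player character 0, it destroys itself first, then casts that character to BP_FirstPersonCharacter.
; It sets shotgun ammo to the maximum, writes the new count directly into the character's WBTempUI text and triggers the character's BorderFlash.
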(event EventBeginPlay)

(event Collision|EventActorBeginOverlap
  (params (OtherActor :type Actor%20Object%20Reference))
  (bind _returnvalue (Game|GetPlayerCharacter 0))
  (if (== OtherActor _returnvalue)
    (Actor|DestroyActor)
    (bind _asbp_first_person_character (Utilities|Casting|CastToBP_FirstPersonCharacter _returnvalue))
    (bind _output_get (Variables|/Game/FirstPerson/Blueprints/BP_FirstPersonCharacter.BP_FirstPersonCharacter_C|SetShotgunAmmo _asbp_first_person_character (Variables|/Game/FirstPerson/Blueprints/BP_FirstPersonCharacter.BP_FirstPersonCharacter_C|GetShotgunMaxAmmo _asbp_first_person_character)))
    (Rendering|Components|TextRender|SetText (Variables|/Game/UI/WB_TempUI.WB_TempUI_C|GetAmmoaAmmount (Variables|/Game/FirstPerson/Blueprints/BP_FirstPersonCharacter.BP_FirstPersonCharacter_C|GetWB_TempUI _asbp_first_person_character)) (Utilities|Text|ToText(Integer) _output_get))
    (Default|BorderFlash _asbp_first_person_character)))

(event EventTick
  (params (DeltaSeconds :type Float%20%28single-precision%29)))

(fn ConstructionScript)