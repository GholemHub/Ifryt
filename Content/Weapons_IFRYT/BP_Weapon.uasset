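; Shotgun weapon Blueprint that handles firing animation, muzzle and impact effects, and bullet spawning.
; BeginPlay sets a dynamic light-beam overlay material on the mesh.
; Fire plays the montage, brightens a lava material, attaches a muzzle flash and drives overlay world position offset through a timeline.
; HitInfo spawns a BP_Bullet aimed at the hit, plus impact Niagara and decal; the delayed material-reset chain is disconnected.
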(event EventBeginPlay
  (bind _returnvalue (Rendering|Material|CreateDynamicMaterialInstance (Variables|Default|GetSK_Shotgun_01) 3 "/Game/Weapons_IFRYT/Shotgun/Materials/M_LightBeams.M_LightBeams" "None" :!class /Script/Engine.PrimitiveComponent))
  (bind _output_get (Variables|Default|SetOverlayMaterial _returnvalue))
  (Rendering|Material|SetOverlayMaterial (Variables|Default|GetSK_Shotgun_01) _output_get :!class /Script/Engine.MeshComponent))

(event Collision|EventActorBeginOverlap
  (params (OtherActor :type Actor%20Object%20Reference)))

(event EventTick
  (params (DeltaSeconds :type Float%20%28single-precision%29)))

(event EventFire
  (Animation|Montage|PlayMontage (Variables|Default|GetSK_Shotgun_01) "/Game/Weapons_IFRYT/Shotgun/Animations/AM_ShGn_Fire_Montage.AM_ShGn_Fire_Montage"
    (:then
      (bind _returnvalue (Rendering|Material|CreateDynamicMaterialInstance (Variables|Default|GetSK_Shotgun_01) 1 "/Game/Weapons_IFRYT/Shotgun/Materials/M_Lava.M_Lava" "None" :!class /Script/Engine.PrimitiveComponent))
      (Variables|Default|SetLava_Mat_Instance _returnvalue)
      (bind _returnvalue_2 (Rendering|Material|GetVectorParameterValue (Variables|Default|GetLava_Mat_Instance) "RedColor" :!class /Script/Engine.MaterialInstanceDynamic))
      (Variables|Default|SetDefault_LavaColor_01 _returnvalue_2)
      (bind _returnvalue_3 (Rendering|Material|GetVectorParameterValue (Variables|Default|GetLava_Mat_Instance) "YellowColor" :!class /Script/Engine.MaterialInstanceDynamic))
      (Variables|Default|SetDefault_LavaColor_02 _returnvalue_3)
      (bind _returnvalue_4 (Rendering|Material|GetScalarParameterValue (Variables|Default|GetLava_Mat_Instance) "Emissive Strenght" :!class /Script/Engine.MaterialInstanceDynamic))
      (Variables|Default|SetDefault_LavaEmission _returnvalue_4)
      (Rendering|Material|SetVectorParameterValue (Variables|Default|GetLava_Mat_Instance) "Red" "(R=1.000000,G=0.014019,B=0.000057,A=1.000000)" :!class /Script/Engine.MaterialInstanceDynamic)
      (Rendering|Material|SetVectorParameterValue (Variables|Default|GetLava_Mat_Instance) "YellowColor" "(R=1.000000,G=0.759493,B=0.000000,A=1.000000)" :!class /Script/Engine.MaterialInstanceDynamic)
      (Rendering|Material|SetScalarParameterValue (Variables|Default|GetLava_Mat_Instance) "Emissive Strenght" 2.0 :!class /Script/Engine.MaterialInstanceDynamic)
      (Niagara|SpawnSystemAttached "/Game/Weapons_IFRYT/Shotgun/VFX/Muzzle_Flash.Muzzle_Flash" (Variables|Default|GetSK_Shotgun_01) "Barrel_Exit" "2.000000,2.000000,-1.000000" "0, 0, 0" "SnapToTargetIncludingScale" true)
      (bind _shoot_material_reaction (Timeline|Timeline PlayFromStart)
        (:Update
          (Rendering|Material|SetScalarParameterValue (Variables|Default|GetOverlayMaterial) "WPO" (Math|Float|Lerp 0.0 2.5 _shoot_material_reaction) :!class /Script/Engine.MaterialInstanceDynamic))))))

(event EventHitInfo
  (params (HitLocation :type Vector :default "0, 0, 0") (HitNormal :type Vector :default "0, 0, 0"))
  (bind _returnvalue (Math|Rotator|MakeRotfromX HitNormal))
  (bind _arrow (Variables|Default|GetArrow))
  (bind _returnvalue_2 (Transformation|GetWorldLocation _arrow))
  (Game|SpawnActorfromClass "/Game/Weapons_IFRYT/BP_Bullet.BP_Bullet_C" (Math|Transform|MakeTransform _returnvalue_2 (Math|Rotator|FindLookatRotation _returnvalue_2 HitLocation) "1.000000,1.000000,1.000000") "AlwaysSpawn" "MultiplyWithRoot" 0 0)
  (Niagara|SpawnSystematLocation "/Game/Weapons_IFRYT/Shotgun/VFX/Impact_Enviro.Impact_Enviro" HitLocation _returnvalue)
  (bind _returnvalue_3 (Rendering|Decal|SpawnDecalatLocation "/Game/Weapons_IFRYT/Shotgun/VFX/HitDecal/Material/M_HitDecal.M_HitDecal" "5.000000,5.000000,5.000000" HitLocation _returnvalue 5.0))
  (Rendering|Components|Decal|SetFadeScreenSize _returnvalue_3 0.0))

(fn ConstructionScript)