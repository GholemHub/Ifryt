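; BP_EnemyTest is a test enemy actor with a placeholder material and a physics-and-dissolve death.
; On BeginPlay it creates one dynamic material instance and applies it to slot 0 of all its static mesh components.
; A one-shot Kill event turns on physics, launches the meshes along the player controller's forward vector, and plays a timeline driving the Dissolve parameter before destroying the actor.
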(event EventBeginPlay
  (bind _returnvalue (Rendering|Material|CreateDynamicMaterialInstance "/Game/_Characters/NPC/Enemy01_Placeholder/Materials/M_EnemyMaterial_Placeholder.M_EnemyMaterial_Placeholder" "None" "None" :!class /Script/Engine.KismetMaterialLibrary))
  (bind _output_get (Variables|Default|SetMaterial _returnvalue))
  (bind _output_get_2 (Variables|Default|SetStaticMeshes (Actor|GetComponentsByClass "/Script/Engine.StaticMeshComponent")))
  (Rendering|Material|SetMaterial _output_get_2 0 _output_get))

(event Collision|EventActorBeginOverlap
  (params (OtherActor :type Actor%20Object%20Reference)))

(event EventTick
  (params (DeltaSeconds :type Float%20%28single-precision%29)))

(event EventKill
  (bind _staticmeshes (Variables|Default|GetStaticMeshes))
  (Utilities|FlowControl|DoOnce false
    (:Completed
      (Physics|SetSimulatePhysics _staticmeshes true)
      (Physics|AddImpulse _staticmeshes (* (Math|Vector|Normalize (Transformation|GetActorForwardVector (Game|GetPlayerController 0)) 0.02) 3e+02) "None" true)
      (bind _dissolve (Timeline|Dissolve PlayFromStart)
        (:Update
          (Rendering|Material|SetScalarParameterValue (Variables|Default|GetMaterial) "Dissolve" _dissolve :!class /Script/Engine.MaterialInstanceDynamic))
        (:Finished
          (Actor|DestroyActor))))))

(fn ConstructionScript)