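; Health component for characters that applies damage and handles death once health runs out, guarded by an IsDead flag.
; When the player (BP_FirstPersonCharacter) dies, the camera blends to the attacker, resolving a VFX projectile to its owner as the kill cam.
; Other owners spawn a random HP, ammo or stamina pickup and receive a KillMessage call.
; Die is an empty stub, and debug prints report the attacker.
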(event EventTick
  (params (DeltaSeconds :type Float%20%28single-precision%29)))

(fn UpdateHP
  (params (Damage :type Float%20%28double-precision%29) (Attacker :type Actor%20Object%20Reference))
  (bind _returnvalue (Components|GetOwner))
  (Development|PrintString (Utilities|GetDisplayName Attacker))
  (if (> (- (Variables|Default|GetHealth) Damage) 0.0)
    (Variables|Default|SetHealth (- (Variables|Default|GetHealth) Damage))
    (elif (not (Variables|Default|GetIsDead))
      (Variables|Default|SetIsDead true)
      (Utilities|Casting|CastToBP_FirstPersonCharacter _returnvalue
        (:then
          (CallFunction|GetAttackerandPlayKillCamera _returnvalue Attacker))
        (:CastFailed
          (CallFunction|SpawnLoot)
          (Class|BPIWeapon|Kill(Message) _returnvalue))))))

(fn Die)

(fn SpawnLoot
  (Game|SpawnActorfromClass (Utilities|Select :Index (Math|Random|RandomIntegerinRange 0 2) :Option%200 "/Game/KojkoTesting/Pickups/BP_HpPickUp.BP_HpPickUp_C" :Option%201 "/Game/KojkoTesting/Pickups/BP_AmmoPickUp.BP_AmmoPickUp_C" :Option%202 "/Game/KojkoTesting/Pickups/BP_StaminaPickUp.BP_StaminaPickUp_C") (Math|Transform|MakeTransform (Transformation|GetActorLocation (Components|GetOwner)) "0, 0, 0" "1.000000,1.000000,1.000000") "Undefined" "MultiplyWithRoot" 0 0)
  (return))

(fn GetAttackerandPlayKillCamera
  (params (Object :type Object%20Object%20Reference) (Attacker :type Actor%20Object%20Reference))
  (bind _asbp_projectile_vfx (Utilities|Casting|CastToBP_Projectile_VFX Attacker)
    (:then
      (Game|Player|SetViewTargetwithBlend (Game|GetPlayerController 0) (Components|GetOwner _asbp_projectile_vfx) 1.0 "VTBlend_EaseInOut" 2.0 false)
      (Development|PrintString (Utilities|GetDisplayName (Components|GetOwner _asbp_projectile_vfx)) true true "(R=0.735544,G=1.000000,B=0.421415,A=1.000000)" 1e+01))
    (:CastFailed
      (Game|Player|SetViewTargetwithBlend (Game|GetPlayerController 0) Attacker 1.0 "VTBlend_EaseInOut" 2.0 false)
      (Development|PrintString (Utilities|String|Append "Attacker is::" (Utilities|GetDisplayName Attacker)) true true "(R=0.000000,G=0.660000,B=1.000000,A=1.000000)" 1e+01))))