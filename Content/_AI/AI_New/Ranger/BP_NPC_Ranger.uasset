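; Ranger enemy NPC that reports see, attack, engage and death events to BP_CombatManager.
; Interface Wait and Attack events forward to AIC_Ranger, while Die notifies the manager and stops the controller's ST.
; Damage feeds BPHealthComponent, and dynamic materials drive a timeline hit overlay.
; Kill launches the static meshes as physics bodies along the player controller's forward vector, ignores pawn collision, then dissolves and destroys the actor.
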(event Custom|OnTakeAnyDamage_Event
  (params (DamagedActor :type Actor%20Object%20Reference) (Damage :type Float%20%28single-precision%29) (DamageType :type Damage%20Type%20Object%20Reference) (InstigatedBy :type Controller%20Object%20Reference) (DamageCauser :type Actor%20Object%20Reference))
  (Default|UpdateHP (Variables|Default|GetBP_HealthComponent) Damage))

(event Custom|UpdateHandleDeath
  ;[0.15 0.15 0.15 0.5] CM_Update
  (Development|PrintString "Handle Death :: LOG1" false false)
  (Default|HandleDeath (Variables|Default|GetCM) self))

(event Custom|Die
  ;[0.15 0.15 0.15 0.5] Die - TODO Add collision death logic (to not step on death body)
  (Utilities|FlowControl|DoOnce false
    (:Completed
      (Class|BPIWeapon|Kill(Message) self)
      (Default|HandleDeath (Variables|Default|GetCM) self)
      (bind _asaic_ranger (Utilities|Casting|CastToAIC_Ranger (Pawn|GetController)))
      (Default|StopST _asaic_ranger))))

(event Custom|UpdateOnSee
  ;[0.15 0.15 0.15 0.5] CM_Update
  (Default|HandleSee (Variables|Default|GetCM) self))

(event Custom|UpdateEngage
  (params (EngagedActor :type Actor%20Object%20Reference))
  ;[0.15 0.15 0.15 0.5] CM_Update
  (Default|EngageWaitingAttacker (Variables|Default|GetCM) EngagedActor))

(event Custom|UpdateOnDontSee
  ;[0.15 0.15 0.15 0.5] CM_Update
  (Default|HandleDontSee (Variables|Default|GetCM) self))

(event Custom|UpdateHandleAttack
  ;[0.15 0.15 0.15 0.5] CM_Update
  (Default|HandleAttackRequest (Variables|Default|GetCM) self))

(event EventBeginPlay
  (bind _returnvalue (Actor|GetActorOfClass "/Game/_AI/AI_New/CombatManager/BP_CombatManager.BP_CombatManager_C"))
  (bind _output_get (Variables|Default|SetCM _returnvalue))
  (Default|HandleAttackRequest _output_get self)
  (EventDispatchers|BindEventtoOnTakeAnyDamage (delegate Custom|OnTakeAnyDamage_Event))
  (bind _returnvalue_2 (Rendering|Material|CreateDynamicMaterialInstance "/Game/_Characters/NPC/Enemy01_Placeholder/Materials/M_EnemyMaterial_Placeholder.M_EnemyMaterial_Placeholder" "None" "None" :!class /Script/Engine.KismetMaterialLibrary))
  (bind _output_get_2 (Variables|Default|SetMaterial _returnvalue_2))
  (bind _output_get_3 (Variables|Default|SetStaticMeshes (Actor|GetComponentsByClass "/Script/Engine.StaticMeshComponent")))
  (Rendering|Material|SetMaterial _output_get_3 0 _output_get_2)
  (bind _returnvalue_3 (Rendering|Material|CreateDynamicMaterialInstance (Variables|Character|GetMesh) 0 "/Game/_Characters/NPC/Materials/Materials/Overlay/M_Overlay.M_Overlay" "None" :!class /Script/Engine.PrimitiveComponent))
  (bind _output_get_4 (Variables|Default|SetOverlayMaterial _returnvalue_3))
  (Rendering|Material|SetOverlayMaterial (Variables|Default|GetStaticMeshes) _output_get_4 :!class /Script/Engine.MeshComponent))

(event EventWait
  (params (AttackTarget :type Actor%20Object%20Reference))
  ;[0.15 0.15 0.15 0.5] Interface
  (Development|PrintString "EVENT WAIT" false false)
  (bind _asaic_ranger (Utilities|Casting|CastToAIC_Ranger (AI|GetAIController self)))
  (Default|WaitEvent _asaic_ranger AttackTarget))

(event EventAttack
  (params (AttackTarget :type Actor%20Object%20Reference))
  ;[0.15 0.15 0.15 0.5] Interface
  (Development|PrintString "Event Attack" false false "(R=0.000000,G=1.000000,B=0.268426,A=1.000000)")
  (bind _asaic_ranger (Utilities|Casting|CastToAIC_Ranger (AI|GetAIController self)))
  (Default|AttackEvent _asaic_ranger AttackTarget))

(event EventKill
  (bind _staticmeshes (Variables|Default|GetStaticMeshes))
  ;[0.15 0.15 0.15 0.5] INTERFACE
  (Utilities|FlowControl|DoOnce false
    (:Completed
      (Physics|SetSimulatePhysics _staticmeshes true)
      (Physics|AddImpulse _staticmeshes (* (Math|Vector|Normalize (Transformation|GetActorForwardVector (Game|GetPlayerController 0)) 0.02) 3e+02) "None" true)
      (Collision|SetCollisionResponsetoChannel _staticmeshes "ECC_Pawn" "ECR_Ignore")
      (Collision|SetCollisionResponsetoChannel (Variables|Collision|GetCapsuleComponent) "ECC_Pawn" "ECR_Ignore")
      (Collision|SetCollisionResponsetoChannel _staticmeshes "ECC_Visibility" "ECR_Ignore")
      (bind _dissolve (Timeline|Timeline PlayFromStart)
        (:Update
          (Rendering|Material|SetScalarParameterValue (Variables|Default|GetMaterial) "Dissolve" _dissolve :!class /Script/Engine.MaterialInstanceDynamic))
        (:Finished
          (Actor|DestroyActor))))))

(event EventHitInfo
  (params (HitLocation :type Vector :default "0, 0, 0") (HitNormal :type Vector :default "0, 0, 0"))
  (bind _newtrack_0 (Timeline|Timeline_0 PlayFromStart)
    (:Update
      (Rendering|Material|SetScalarParameterValue (Variables|Default|GetOverlayMaterial) "MaterialVisibility" _newtrack_0 :!class /Script/Engine.MaterialInstanceDynamic))))

(fn ConstructionScript)

(fn SetupUI)

(fn ShowEnemyUI
  (Rendering|SetVisibility (Variables|Default|GetWidget) true true))

(fn HideEnemyUI
  (Rendering|SetVisibility (Variables|Default|GetWidget) false true))