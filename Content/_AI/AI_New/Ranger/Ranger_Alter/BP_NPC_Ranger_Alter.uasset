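; Alternate Ranger enemy NPC that fires projectiles at the player and reports to the wave manager when killed.
; Attack spawns a player-aimed projectile behind a brief cooldown, while damage feeds the health component and HitInfo animates an overlay material as hit feedback.
; Kill stops the StateTree, turns meshes into impulse-driven physics debris and dissolves them before destroying the actor and requesting another spawn.
; A separate Die path hands off to CM.HandleDeath and casts to AIC_Ranger, not AIC_Ranger_Alter.
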(event Custom|OnTakeAnyDamage_Event
  (params (DamagedActor :type Actor%20Object%20Reference) (Damage :type Float%20%28single-precision%29) (DamageType :type Damage%20Type%20Object%20Reference) (InstigatedBy :type Controller%20Object%20Reference) (DamageCauser :type Actor%20Object%20Reference))
  (Default|UpdateHP (Variables|Default|GetBP_HealthComponent) Damage))

(event Custom|PlayVFX
  (Components|Activation|Activate (Variables|Default|GetFX_Spawning) false))

(event Custom|SetVisibility
  (Rendering|SetVisibility (Variables|Character|GetMesh) true true))

(event Custom|Die
  ;[0.15 0.15 0.15 0.5] Die - TODO Add collision death logic (to not step on death body)
  (Utilities|FlowControl|DoOnce false
    (:Completed
      (Class|BPIWeapon|Kill(Message) self)
      (Default|HandleDeath (Variables|Default|GetCM) self)
      (bind _asaic_ranger (Utilities|Casting|CastToAIC_Ranger (Pawn|GetController)))
      (Default|StopST _asaic_ranger))))

(event Custom|Attack
  (bind _firepoint (Variables|Default|GetFirePoint))
  (bind _returnvalue (Transformation|GetWorldLocation _firepoint))
  ;[0.15 0.15 0.15 0.5] Attack
  (if (not (Variables|Default|GetbHasFired))
    (Variables|Default|SetbHasFired true)
    (bind _returnvalue_2 (Game|SpawnActorfromClass "/Game/_AI/AI_New/Ranger/Ranger_Alter/BP_Projectile_Ranger.BP_Projectile_Ranger_C" (Math|Transform|MakeTransform _returnvalue (Math|Rotator|FindLookatRotation _returnvalue (Transformation|GetActorLocation (Game|Player|GetPlayerPawn 0))) "1.000000,1.000000,1.000000") "AdjustIfPossibleButAlwaysSpawn" "MultiplyWithRoot" 0 self))
    (Variables|/Script/Engine.MovementComponent|SetVelocity (Actor|GetComponentbyClass _returnvalue_2 "/Script/Engine.ProjectileMovementComponent") (* (Math|Vector|Normalize (- (Transformation|GetActorLocation (Game|Player|GetPlayerPawn 0)) (Transformation|GetWorldLocation (Variables|Default|GetFirePoint)))) 1.5e+03))
    (Development|PrintString "Fire in ranger Alter")
    (Utilities|FlowControl|Delay 0.2)
    (Variables|Default|SetbHasFired false)))

(event EventBeginPlay
  (EventDispatchers|BindEventtoOnTakeAnyDamage (delegate Custom|OnTakeAnyDamage_Event))
  (bind _returnvalue (Rendering|Material|CreateDynamicMaterialInstance "/Game/_Characters/NPC/GotF_Ranger/Materials/M_Enemy_MasterMaterial.M_Enemy_MasterMaterial" "None" "None" :!class /Script/Engine.KismetMaterialLibrary))
  (bind _output_get (Variables|Default|SetMaterial _returnvalue))
  (bind _output_get_2 (Variables|Default|SetStaticMeshes (Actor|GetComponentsByClass "/Script/Engine.StaticMeshComponent")))
  (Rendering|Material|SetMaterial _output_get_2 0 _output_get)
  (bind _returnvalue_2 (Rendering|Material|CreateDynamicMaterialInstance (Variables|Character|GetMesh) 0 "/Game/_Characters/NPC/Special_Materials/Materials/Overlay/M_Overlay.M_Overlay" "None" :!class /Script/Engine.PrimitiveComponent))
  (bind _output_get_3 (Variables|Default|SetOverlayMaterial _returnvalue_2))
  (Rendering|Material|SetOverlayMaterial (Variables|Default|GetStaticMeshes) _output_get_3 :!class /Script/Engine.MeshComponent))

(event EventFire)

(event EventKill
  (bind _staticmeshes (Variables|Default|GetStaticMeshes))
  ;[0.15 0.15 0.15 0.5] INTERFACE
  (Utilities|FlowControl|DoOnce false
    (:Completed
      (bind _asaic_ranger_alter (Utilities|Casting|CastToAIC_Ranger_Alter (Pawn|GetController)))
      (Default|StopST _asaic_ranger_alter)
      (Physics|SetSimulatePhysics _staticmeshes true)
      (Utilities|CheckifHasPhysics _staticmeshes
        (:then
          (Physics|AddImpulse _staticmeshes (* (Math|Vector|Normalize (Transformation|GetActorForwardVector (Game|GetPlayerController 0)) 0.02) 3e+02) "None" true))
        (:false
          _))
      (Collision|SetCollisionResponsetoChannel _staticmeshes "ECC_Pawn" "ECR_Ignore")
      (Collision|SetCollisionResponsetoChannel (Variables|Collision|GetCapsuleComponent) "ECC_Pawn" "ECR_Ignore")
      (Collision|SetCollisionResponsetoChannel _staticmeshes "ECC_Visibility" "ECR_Ignore")
      (bind _dissolve (Timeline|Timeline_1 PlayFromStart)
        (:Update
          (Rendering|Material|SetScalarParameterValue (Variables|Default|GetMaterial) "Dissolve" _dissolve :!class /Script/Engine.MaterialInstanceDynamic))
        (:Finished
          (Actor|DestroyActor)
          (bind _returnvalue (Actor|GetActorOfClass "/Game/_AI/AI_New/CombatManager/BP_WaweManager_alter.BP_WaweManager_alter_C"))
          (Variables|/Game/_AI/AI_New/CombatManager/BP_WaweManager_alter.BP_WaweManager_alter_C|SetKillsToFinish _returnvalue (- (Variables|/Game/_AI/AI_New/CombatManager/BP_WaweManager_alter.BP_WaweManager_alter_C|GetKillsToFinish _returnvalue) 1))
          (Default|SpawnNewEnemy _returnvalue))))))

(event EventHitInfo
  (params (HitLocation :type Vector :default "0, 0, 0") (HitNormal :type Vector :default "0, 0, 0"))
  (bind _newtrack_0 (Timeline|Timeline_0 PlayFromStart)
    (:Update
      (Rendering|Material|SetScalarParameterValue (Variables|Default|GetOverlayMaterial) "MaterialVisibility" _newtrack_0 :!class /Script/Engine.MaterialInstanceDynamic))))

(fn ConstructionScript)

(fn SetupUI)

(fn ShowEnemyUI
  (Rendering|SetVisibility (Variables|Default|GetWidget) true true))

(fn HideEnemyUI
  (Rendering|SetVisibility (Variables|Default|GetWidget) false true))