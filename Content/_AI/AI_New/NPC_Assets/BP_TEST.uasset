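; Test NPC Blueprint for pushing values into its AIC_Test AI controller.
; Tick flip-flops and prints a bool, then sends it through UpdateBool1; Log alternates a tag between Test.One and Test.Two for the controller, and UpdateTag clears the controller's tag.
; ShowEnemyUI and HideEnemyUI toggle widget visibility.
; State events and SetupUI are empty stubs, with leftover AIState and debug print logic left unconnected.
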(event Custom|UpdateTag
  (bind _asaic_test (Utilities|Casting|CastToAIC_Test (AI|GetAIController 0)))
  (Variables|/Game/_AI/AI_New/AIC_Test.AIC_Test_C|SetTAG_AIC_Test _asaic_test ""))

(event Custom|Server_ChangeState
  ;[0.15 0.15 0.15 0.5] states
)

(event Custom|Log
  (Utilities|FlowControl|FlipFlop
    (:A
      (Variables|Default|SetTag "(TagName=\"Test.One\")"))
    (:B
      (Variables|Default|SetTag "(TagName=\"Test.Two\")")))
  (bind _asaic_test (Utilities|Casting|CastToAIC_Test (AI|GetAIController self)))
  (Default|UpdateTag _asaic_test (Variables|Default|GetTag)))

(event Custom|ChangeState
  ;[0.15 0.15 0.15 0.5] states
)

(event EventBeginPlay)

(event EventTick
  (params (DeltaSeconds :type Float%20%28single-precision%29))
  (Utilities|FlowControl|FlipFlop
    (:A
      (Variables|Default|SetBoolParam_BP false)
      (Development|PrintString (Utilities|String|ToString(Boolean) (Variables|Default|GetBoolParam_BP))))
    (:B
      (Variables|Default|SetBoolParam_BP true)
      (Development|PrintString (Utilities|String|ToString(Boolean) (Variables|Default|GetBoolParam_BP)))))
  (bind _asaic_test (Utilities|Casting|CastToAIC_Test (AI|GetAIController self))
    (:then
      (Default|UpdateBool1 _asaic_test (Variables|Default|GetBoolParam_BP)))
    (:CastFailed
      (Development|PrintString "Hello"))))

(event EventWait
  (params (AttakTarget :type Actor%20Object%20Reference))
  ;[0.15 0.15 0.15 0.5] states
)

(event EventRetreat
  ;[0.15 0.15 0.15 0.5] states
)

(fn ConstructionScript)

(fn SetupUI)

(fn ShowEnemyUI
  (Rendering|SetVisibility (Variables|Default|GetWidget) true true))

(fn HideEnemyUI
  (Rendering|SetVisibility (Variables|Default|GetWidget) false true))