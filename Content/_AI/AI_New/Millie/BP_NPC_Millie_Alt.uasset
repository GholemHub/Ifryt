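; Alternate Millie NPC that damages the player with a delayed, close-range attack while spinning its mesh.
; A sphere overlap sets a target flag while the first-person character is inside.
; AttackEvent, which nothing in this graph calls, waits briefly, then applies damage to the player pawn only if that flag is still set.
; After a hit, a timeline drives incremental yaw rotation on the mesh at a curve-controlled rate.
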(event OnComponentBeginOverlap(Sphere)
  (params (OverlappedComponent :type Primitive%20Component%20Object%20Reference) (OtherActor :type Actor%20Object%20Reference) (OtherComp :type Primitive%20Component%20Object%20Reference) (OtherBodyIndex :type Integer) (bFromSweep :type Boolean) (SweepResult :type Hit%20Result%20Structure%20%28by%20ref%29))
  ;[0.07429 0.07429 0.07812] ATTACKING
  (Utilities|Casting|CastToBP_FirstPersonCharacter OtherActor)
  (Variables|Default|SetHas%20Target true))

(event OnComponentEndOverlap(Sphere)
  (params (OverlappedComponent :type Primitive%20Component%20Object%20Reference) (OtherActor :type Actor%20Object%20Reference) (OtherComp :type Primitive%20Component%20Object%20Reference) (OtherBodyIndex :type Integer))
  ;[0.07429 0.07429 0.07812] ATTACKING
  (Utilities|Casting|CastToBP_FirstPersonCharacter OtherActor)
  (Variables|Default|SetHas%20Target false))

(event Custom|AttackEvent
  ;[0.07429 0.07429 0.07812] ATTACKING
  (Utilities|FlowControl|Delay 1.0)
  (if (Variables|Default|GetHas%20Target)
    (Game|Damage|ApplyDamage (Game|Player|GetPlayerPawn 0) 2e+01 0 0)
    (bind _newtrack_0 (Timeline|Timeline PlayFromStart)
      (:Update
        (Transformation|AddLocalRotation (Variables|Character|GetMesh) (Math|Rotator|MakeRotator 0.0 0.0 (Math|Float|Lerp 2.0 12.0 _newtrack_0)) false false)))))

(event EventBeginPlay)

(event Collision|EventActorBeginOverlap
  (params (OtherActor :type Actor%20Object%20Reference)))

(event EventTick
  (params (DeltaSeconds :type Float%20%28single-precision%29)))

(fn ConstructionScript)