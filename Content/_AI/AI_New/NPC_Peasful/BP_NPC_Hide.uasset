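; Peaceful hiding NPC that takes damage, drops ammo on death and has an enemy UI widget that can be shown or hidden.
; Any damage is forwarded to BPHealthComponent.
; Die runs once: it ragdolls the mesh with an impulse along the player controller's forward, calls StopST on AIC_EQS_Hide, spawns BP_AmmoPickUp, then destroys the actor after a delay.
; SetupUI is empty, and death collision handling is still a TODO.
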(event Custom|OnTakeAnyDamage_Event
  (params (DamagedActor :type Actor%20Object%20Reference) (Damage :type Float%20%28single-precision%29) (DamageType :type Damage%20Type%20Object%20Reference) (InstigatedBy :type Controller%20Object%20Reference) (DamageCauser :type Actor%20Object%20Reference))
  (Default|UpdateHP (Variables|Default|GetBP_HealthComponent) Damage))

(event Custom|Die
  (bind _mesh (Variables|Character|GetMesh))
  ;[0.15 0.15 0.15 0.5] Die - TODO Add collision death logic (to not step on death body)
  (Utilities|FlowControl|DoOnce false
    (:Completed
      (Physics|SetSimulatePhysics _mesh true)
      (Physics|AddImpulse _mesh (* (Math|Vector|Normalize (Transformation|GetActorForwardVector (Game|GetPlayerController 0)) 0.02) 3e+02) "None" true)
      (bind _asaic_eqs_hide (Utilities|Casting|CastToAIC_EQS_Hide (Pawn|GetController)))
      (Default|StopST _asaic_eqs_hide)
      (Game|SpawnActorfromClass "/Game/KojkoTesting/Pickups/BP_AmmoPickUp.BP_AmmoPickUp_C" (Transformation|GetActorTransform) "AdjustIfPossibleButAlwaysSpawn" "MultiplyWithRoot" 0 0)
      (Utilities|FlowControl|Delay 5.0)
      (Actor|DestroyActor))))

(event EventBeginPlay
  (EventDispatchers|BindEventtoOnTakeAnyDamage (delegate Custom|OnTakeAnyDamage_Event)))

(fn ConstructionScript)

(fn SetupUI)

(fn ShowEnemyUI
  (Rendering|SetVisibility (Variables|Default|GetWidget) true true))

(fn HideEnemyUI
  (Rendering|SetVisibility (Variables|Default|GetWidget) false true))