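; BP_CombatManager limits how many AI attack one target at once, defaulting to the player and reading the cap from that target.
; Attack and sight requests fill the Attackers list, then overflow into WaitingAttackers, with Attack or Wait messages sent to each.
; An attacker's death promotes the first waiter, while the target's death sets everyone waiting and clears both lists.
; Losing sight removes that AI and sends Wait without promoting a replacement.
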(event EventBeginPlay
  (Variables|Default|GetAttackTarget
    (:then
      _)
    (:else
      (Variables|Default|SetAttackTarget (Game|GetPlayerCharacter 0))))
  (bind _value (Class|BPIAttackTarget|GetMaxAttackerCount(Message) (Variables|Default|GetAttackTarget)))
  (Variables|Default|SetMaxAttackersCount _value))

(fn ConstructionScript)

(fn HandleAttackRequest
  (params (Attacker :type Actor%20Object%20Reference))
  (if (!= Attacker (Variables|Default|GetAttackTarget))
    (if (< (Utilities|Array|Length (Variables|Default|GetAttackers)) (Variables|Default|GetMaxAttackersCount))
      (Utilities|Array|AddUnique (Variables|Default|GetAttackers) Attacker)
      (Class|BPIAttacker|Attack(Message) Attacker (Variables|Default|GetAttackTarget))
      (else
        (Utilities|Array|AddUnique (Variables|Default|GetWaitingAttackers) Attacker)
        (Class|BPIAttacker|Wait(Message) Attacker (Variables|Default|GetAttackTarget))))))

(fn HandleDeath
  (params (ActorRef :type Actor%20Object%20Reference))
  (bind _attackers (Variables|Default|GetAttackers))
  (if (== ActorRef (Variables|Default|GetAttackTarget))
    (Utilities|Array|AppendArray _attackers (Variables|Default|GetWaitingAttackers))
    (for _array_element _attackers
      (Class|BPIAttacker|Wait(Message) _array_element (Variables|Default|GetAttackTarget)))
    (Utilities|Array|Clear (Variables|Default|GetAttackers))
    (Utilities|Array|Clear (Variables|Default|GetWaitingAttackers))
    (else
      (Development|PrintString "Death::LOG::1")
      (if (Utilities|Array|ContainsItem (Variables|Default|GetAttackers) ActorRef)
        (Utilities|Array|RemoveItem (Variables|Default|GetAttackers) ActorRef)
        (CallFunction|EngageWaitingAttacker)
        (elif (Utilities|Array|ContainsItem (Variables|Default|GetWaitingAttackers) ActorRef)
          (Utilities|Array|RemoveItem (Variables|Default|GetWaitingAttackers) ActorRef))))))

(fn EngageWaitingAttacker
  (params (EngagedActor :type Actor%20Object%20Reference))
  (bind _waitingattackers (Variables|Default|GetWaitingAttackers))
  (bind _output (Utilities|Array|Get(acopy) _waitingattackers))
  (Utilities|IsValid _output
    (:Is%20Valid
      (bind _output_get (LocalVariables|SetWaitingAttacker _output))
      (Utilities|Array|RemoveItem (Variables|Default|GetWaitingAttackers) _output_get)
      (Utilities|Array|AddUnique (Variables|Default|GetAttackers) _output_get)
      (Development|PrintString "Hello")
      (Class|BPIAttacker|Attack(Message) (LocalVariables|GetWaitingAttacker) (Variables|Default|GetAttackTarget)))))

(fn HandleSee
  (params (Attacker :type Actor%20Object%20Reference))
  (if (< (Utilities|Array|Length (Variables|Default|GetAttackers)) (Variables|Default|GetMaxAttackersCount))
    (Utilities|Array|AddUnique (Variables|Default|GetAttackers) Attacker)
    (Class|BPIAttacker|Attack(Message) Attacker (Variables|Default|GetAttackTarget))
    (else
      (Utilities|Array|AddUnique (Variables|Default|GetWaitingAttackers) Attacker)
      (Class|BPIAttacker|Wait(Message) Attacker (Variables|Default|GetAttackTarget)))))

(fn HandleDontSee
  (params (Attacker :type Actor%20Object%20Reference))
  (bind _returnvalue (Utilities|Array|RemoveItem (Variables|Default|GetAttackers) Attacker))
  (if _returnvalue
    (Class|BPIAttacker|Wait(Message) Attacker (Variables|Default|GetAttackTarget) :!label _label)
    (else
      (bind _returnvalue_2 (Utilities|Array|RemoveItem (Variables|Default|GetWaitingAttackers) Attacker))
      (if _returnvalue_2
        (goto _label)))))