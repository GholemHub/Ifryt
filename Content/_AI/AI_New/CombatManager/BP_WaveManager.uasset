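; BP_WaveManager spawns escalating enemy waves at random navigable points within a radius of itself.
; Tick sets CanSpawn by whether instances of each listed class exist, so only the last class checked counts.
; A looping timer spawns the first listed class when allowed and increments the enemy count.
; Each firing doubles WaitingTime, but the timer is never reset, so its interval stays fixed.
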(event Custom|Spawn
  (CallFunction|SpawnNewEnemyes)
  (Variables|Default|SetWaitingTime (+ (Variables|Default|GetWaitingTime) (Variables|Default|GetWaitingTime))))

(event EventBeginPlay
  (Utilities|Time|SetTimerbyEvent (delegate Custom|Spawn) (Variables|Default|GetWaitingTime) true false 1.0))

(event Collision|EventActorBeginOverlap
  (params (OtherActor :type Actor%20Object%20Reference)))

(event EventTick
  (params (DeltaSeconds :type Float%20%28single-precision%29))
  (for _array_element (Variables|Default|GetActorsToSpawn)
    (bind _outactors (Actor|GetAllActorsOfClass _array_element))
    (if (== (Utilities|Array|Length _outactors) 0)
      (Variables|Default|SetCanSpawn true)
      (else
        (Variables|Default|SetCanSpawn false)))))

(fn ConstructionScript)

(fn SpawnNewEnemyes
  (bind _returnvalue (Transformation|GetActorTransform))
  (if (Variables|Default|GetCanSpawn)
    (for _index (range 0 (Variables|Default|GetNumberOfEnemy))
      (bind _randomlocation (Class|NavigationSystemV1|GetRandomLocationinNavigableRadius (Transformation|GetActorLocation) (Variables|Default|GetRadius) 0 0))
      (Game|SpawnActorfromClass (Utilities|Array|Get(acopy) (Variables|Default|GetActorsToSpawn) (Math|Random|RandomInteger 0)) (Math|Transform|MakeTransform _randomlocation (.rotation _returnvalue) (.scale _returnvalue)) "Undefined" "MultiplyWithRoot" 0 0))
    (bind _output_get (Variables|Default|SetNumberOfEnemy (+ (Variables|Default|GetNumberOfEnemy) 1)))
    (Development|PrintString (Utilities|String|ToString(Integer) _output_get))))