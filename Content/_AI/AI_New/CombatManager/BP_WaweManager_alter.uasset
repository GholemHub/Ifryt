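; Wave manager that spawns random Millie or Ranger enemies at reachable navmesh points within a radius.
; A player overlap, or OnStart for boss waves, activates it once, raises the player's LevelStage and spawns the opening batch.
; SpawnNewEnemy1 spawns until the kill quota is covered, then, when none remain, opens a door or notifies BP_Boss.
; Tick prints debug enemy counts; EnemyCounter is never incremented here.
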(event OnComponentBeginOverlap(Box)
  (params (OverlappedComponent :type Primitive%20Component%20Object%20Reference) (OtherActor :type Actor%20Object%20Reference) (OtherComp :type Primitive%20Component%20Object%20Reference) (OtherBodyIndex :type Integer) (bFromSweep :type Boolean) (SweepResult :type Hit%20Result%20Structure%20%28by%20ref%29))
  (if (not (Variables|Default|GetIsBoss?))
    (if (not (Variables|Default|GetActivated))
      (Utilities|FlowControl|DoOnce false
        (:Completed
          (Variables|Default|SetActivated true)
          (bind _asbp_first_person_character (Utilities|Casting|CastToBP_FirstPersonCharacter OtherActor))
          (Variables|/Game/FirstPerson/Blueprints/BP_FirstPersonCharacter.BP_FirstPersonCharacter_C|SetLevelStage _asbp_first_person_character (+ (Variables|/Game/FirstPerson/Blueprints/BP_FirstPersonCharacter.BP_FirstPersonCharacter_C|GetLevelStage _asbp_first_person_character) 1))
          (for _index (range 0 (- (Variables|Default|GetSpawnFromStart) 1))
            (CallFunction|SpawnNewEnemy1)))))))

(event Custom|OnStart
  (if (not (Variables|Default|GetActivated))
    (Utilities|FlowControl|DoOnce false
      (:Completed
        (Variables|Default|SetActivated true)
        (bind _asbp_first_person_character (Utilities|Casting|CastToBP_FirstPersonCharacter (stale OnComponentBeginOverlap(Box) OtherActor)))
        (Variables|/Game/FirstPerson/Blueprints/BP_FirstPersonCharacter.BP_FirstPersonCharacter_C|SetLevelStage _asbp_first_person_character (+ (Variables|/Game/FirstPerson/Blueprints/BP_FirstPersonCharacter.BP_FirstPersonCharacter_C|GetLevelStage _asbp_first_person_character) 1))
        (for _index (range 0 (- (Variables|Default|GetSpawnFromStart) 1))
          (CallFunction|SpawnNewEnemy1))))))

(event Custom|OnDone
  (bind _doortoopen (Variables|Default|GetDoorToOpen))
  (if (Variables|Default|GetIsBoss?)
    (bind _returnvalue (Actor|GetActorOfClass "/Game/KojkoTesting/Blueprints/Boss/BP_Boss.BP_Boss_C"))
    (Default|EnemiesCleared _returnvalue)
    (else
      (Utilities|IsValid _doortoopen
        (:Is%20Valid
          (Default|OnOpenEvent _doortoopen))))))

(event EventTick
  (params (DeltaSeconds :type Float%20%28single-precision%29))
  (if (Variables|Default|GetActivated)
    (bind _outactors (Actor|GetAllActorsOfClass "/Game/_AI/AI_New/Ranger/Ranger_Alter/BP_NPC_Ranger_Alter.BP_NPC_Ranger_Alter_C"))
    (bind _output_get (Variables|Default|SetRangeEnemyCount (Utilities|Array|Length _outactors)))
    (bind _outactors_2 (Actor|GetAllActorsOfClass "/Game/_AI/AI_New/Millie/Millie_Alter/BP_NPC_Millie_Alter.BP_NPC_Millie_Alter_C"))
    (bind _output_get_2 (Variables|Default|SetMillieEnemyCount (Utilities|Array|Length _outactors_2)))
    (Development|PrintString (Utilities|String|Append "Millie:" (Utilities|String|ToString(Integer) _output_get_2) ":: Range::" (Utilities|String|ToString(Integer) _output_get) "::Kills To Finish::::::::" (Utilities|String|ToString(Integer) (Variables|Default|GetKillsToFinish)) "::counter Enemy::" (Utilities|String|ToString(Integer) (Variables|Default|GetEnemyCounter))) true true "(R=0.000000,G=0.660000,B=1.000000,A=1.000000)" 0.0)))

(fn ConstructionScript
  (Components|Sphere|SetSphereRadius (Variables|Default|GetSphere1) (Variables|Default|GetRadius) true))

(fn SpawnNewEnemy1
  (bind _activated (Variables|Default|GetActivated))
  (Development|PrintString (Utilities|String|ToString(Boolean) _activated) false)
  (if _activated
    (if (<= (+ (Variables|Default|GetEnemyCounter) (Variables|Default|GetSpawnFromStart)) (Variables|Default|GetKillsToFinish))
      (bind _randomlocation (AI|Navigation|GetRandomReachablePointinRadius (Transformation|GetActorLocation) (Variables|Default|GetRadius) 0 "/Script/NavigationSystem.NavigationQueryFilter"))
      (Development|PrintString (Utilities|String|ToString(Vector) _randomlocation) false true "(R=0.000000,G=0.660000,B=1.000000,A=1.000000)" 1e+01)
      (AI|SpawnAIFromClass (Utilities|Select :Index (Math|Random|RandomIntegerinRange 0 1) :Option%200 "/Game/_AI/AI_New/Millie/Millie_Alter/BP_NPC_Millie_Alter.BP_NPC_Millie_Alter_C" :Option%201 "/Game/_AI/AI_New/Ranger/Ranger_Alter/BP_NPC_Ranger_Alter.BP_NPC_Ranger_Alter_C") 0 _randomlocation "0, 0, 0" true 0)
      (else
        (bind _outactors (Actor|GetAllActorsOfClass "/Game/_AI/AI_New/Millie/Millie_Alter/AIC_Millie_Alter.AIC_Millie_Alter_C"))
        (bind _outactors_2 (Actor|GetAllActorsOfClass "/Game/_AI/AI_New/Ranger/Ranger_Alter/BP_NPC_Ranger_Alter.BP_NPC_Ranger_Alter_C"))
        (if (== (+ (Utilities|Array|Length _outactors_2) (Utilities|Array|Length _outactors)) 0)
          (Development|PrintString "Done")
          (CallFunction|OnDone)
          (else
            (Development|PrintString "UNDONE")))))))