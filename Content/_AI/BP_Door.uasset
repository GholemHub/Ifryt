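; Door actor that sinks below its starting height to open and rises back to close, with two meshes constantly counter-rotating.
; Open and close events, gated by IsOpen, each drive a timeline lerping actor height from the Z cached on BeginPlay.
; Spawn effects fire as opening starts and closing finishes, with a delayed stone sound behind a DoOnce in each direction.
; Doors flagged IsOpen begin lowered.
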(event Custom|OnOpenEvent
  (bind _returnvalue (Transformation|GetActorLocation))
  (bind _z (Variables|Default|GetZ))
  (if (not (Variables|Default|GetIsOpen))
    (Components|Activation|Activate (Variables|Default|GetFX_Spawning) false)
    (bind _dissolve (Timeline|Timeline PlayFromStart)
      (:Update
        (Transformation|SetActorRelativeLocation (Math|Vector|MakeVector (.x _returnvalue) (.y _returnvalue) (Math|Float|Lerp _z (+ _z -1.5e+03) _dissolve)))
        (Utilities|FlowControl|DoOnce false
          (:Completed
            (Utilities|FlowControl|Delay 1.0)
            (Audio|PlaySoundatLocation "/Game/_AI/Sounds/Stone.Stone" (Transformation|GetActorLocation) "0, 0, 0" 1.0 1.0 0.0 0 0 0 0))))
      (:Finished
        (Variables|Default|SetIsOpen true)))))

(event Custom|OnCloseEvent
  (bind _returnvalue (Transformation|GetActorLocation))
  (bind _z (Variables|Default|GetZ))
  (if (Variables|Default|GetIsOpen)
    (bind _dissolve (Timeline|Timeline_0 Play)
      (:Update
        (Transformation|SetActorRelativeLocation (Math|Vector|MakeVector (.x _returnvalue) (.y _returnvalue) (Math|Float|Lerp (+ _z -1.5e+03) _z _dissolve)))
        (Utilities|FlowControl|DoOnce false
          (:Completed
            (Utilities|FlowControl|Delay 1.0)
            (Audio|PlaySoundatLocation "/Game/_AI/Sounds/Stone.Stone" (Transformation|GetActorLocation) "0, 0, 0" 1.0 1.0 0.0 0 0 0 0))))
      (:Finished
        (Components|Activation|Activate (Variables|Default|GetFX_Spawning) false)
        (Variables|Default|SetIsOpen false)))))

(event Custom|FirstOpen)

(event EventBeginPlay
  (bind _returnvalue (Transformation|GetActorLocation))
  (Variables|Default|SetZ (.z (Transformation|GetActorLocation)))
  (if (Variables|Default|GetIsOpen)
    (Transformation|SetActorRelativeLocation (Math|Vector|MakeVector (.x _returnvalue) (.y _returnvalue) (+ (Variables|Default|GetZ) -1.5e+03)))))

(event EventTick
  (params (DeltaSeconds :type Float%20%28single-precision%29))
  (Transformation|AddRelativeRotation (Variables|Default|GetStaticMesh4) (Math|Rotator|MakeRotator 0.0 0.0 1.0) false false)
  (Transformation|AddRelativeRotation (Variables|Default|GetStaticMesh3) (Math|Rotator|MakeRotator 0.0 0.0 -1.0) false false))

(fn ConstructionScript)