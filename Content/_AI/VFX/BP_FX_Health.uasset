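; BP_FX_Health is a particle-driven health pickup that applies negative damage, presumably as healing, when the player touches it.
; On BeginPlay it passes itself to its Niagara system as the export target for particle data.
; Each data callback moves a collision sphere to just above the exported particle positions, ending at the last one.
; When the player character overlaps that sphere, the pickup applies the negative damage and destroys itself.
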(event OnComponentBeginOverlap(Sphere)
  (params (OverlappedComponent :type Primitive%20Component%20Object%20Reference) (OtherActor :type Actor%20Object%20Reference) (OtherComp :type Primitive%20Component%20Object%20Reference) (OtherBodyIndex :type Integer) (bFromSweep :type Boolean) (SweepResult :type Hit%20Result%20Structure%20%28by%20ref%29))
  (if (== OtherActor (Game|GetPlayerCharacter 0))
    (Game|Damage|ApplyDamage OtherActor -25.0 0 0)
    (Actor|DestroyActor)))

(event Collision|EventActorBeginOverlap
  (params (OtherActor :type Actor%20Object%20Reference)))

(event EventTick
  (params (DeltaSeconds :type Float%20%28single-precision%29)))

(event EventParticleData
  (params (Data :type Array%20of%20Basic%20Particle%20Data%20Structures) (NiagaraSystem :type Niagara%20System%20Object%20Reference) (SimulationPositionOffset :type Vector%20%28by%20ref%29 :default "0, 0, 0"))
  (for _array_element Data
    (Transformation|SetWorldLocation (Variables|Default|GetSphere) (Math|Vector|MakeVector (.x (.Position (Utilities|Struct|BreakBasicParticleData _array_element))) (.y (.Position (Utilities|Struct|BreakBasicParticleData _array_element))) (+ (.z (.Position (Utilities|Struct|BreakBasicParticleData _array_element))) 5e+01)) false false)))

(event EventBeginPlay
  (Niagara|SetNiagaraVariable(Object) (Variables|Default|GetNiagara) "User.Blueprint" self))

(fn ConstructionScript)