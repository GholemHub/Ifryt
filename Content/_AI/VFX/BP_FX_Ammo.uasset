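; BP_FX_Ammo is a Niagara-based ammo pickup that refills the player's shotgun ammo to max.
; It passes itself to Niagara as the export callback, and received particle data moves the collision sphere to just above each particle position in turn.
; When the player overlaps the sphere, the actor destroys itself, updates the ammo, HUD text and calls the character's border flash.
; A disconnected negative-damage branch never runs.
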(event OnComponentBeginOverlap(Sphere)
  (params (OverlappedComponent :type Primitive%20Component%20Object%20Reference) (OtherActor :type Actor%20Object%20Reference) (OtherComp :type Primitive%20Component%20Object%20Reference) (OtherBodyIndex :type Integer) (bFromSweep :type Boolean) (SweepResult :type Hit%20Result%20Structure%20%28by%20ref%29))
  (bind _returnvalue (Game|GetPlayerCharacter 0))
  (if (== OtherActor _returnvalue)
    (Actor|DestroyActor)
    (bind _asbp_first_person_character (Utilities|Casting|CastToBP_FirstPersonCharacter _returnvalue))
    (bind _output_get (Variables|/Game/FirstPerson/Blueprints/BP_FirstPersonCharacter.BP_FirstPersonCharacter_C|SetShotgunAmmo _asbp_first_person_character (Variables|/Game/FirstPerson/Blueprints/BP_FirstPersonCharacter.BP_FirstPersonCharacter_C|GetShotgunMaxAmmo _asbp_first_person_character)))
    (Rendering|Components|TextRender|SetText (Variables|/Game/UI/WB_TempUI.WB_TempUI_C|GetAmmoaAmmount (Variables|/Game/FirstPerson/Blueprints/BP_FirstPersonCharacter.BP_FirstPersonCharacter_C|GetWB_TempUI _asbp_first_person_character)) (Utilities|Text|ToText(Integer) _output_get))
    (Default|BorderFlash _asbp_first_person_character)))

(event Collision|EventActorBeginOverlap
  (params (OtherActor :type Actor%20Object%20Reference)))

(event EventTick
  (params (DeltaSeconds :type Float%20%28single-precision%29)))

(event EventParticleData
  (params (Data :type Array%20of%20Basic%20Particle%20Data%20Structures) (NiagaraSystem :type Niagara%20System%20Object%20Reference) (SimulationPositionOffset :type Vector%20%28by%20ref%29 :default "0, 0, 0"))
  (for _array_element Data
    (Transformation|SetWorldLocation (Variables|Default|GetSphere) (Math|Vector|MakeVector (.x (.Position (Utilities|Struct|BreakBasicParticleData _array_element))) (.y (.Position (Utilities|Struct|BreakBasicParticleData _array_element))) (+ (.z (.Position (Utilities|Struct|BreakBasicParticleData _array_element))) 5e+01)) false false)))

(event EventBeginPlay
  (Niagara|SetNiagaraVariable(Object) (Variables|Default|GetNiagara) "User.Blueprint" self))

(fn ConstructionScript)