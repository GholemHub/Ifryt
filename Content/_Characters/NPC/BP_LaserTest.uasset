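; BP_LaserTest is a test actor that shows a continuously rotating laser beam.
; Each tick it yaws a Sphere component at RotationSpeed scaled by delta time, then line traces on the Visibility channel along the sphere's forward vector.
; The impact point, or the trace end when nothing blocks, feeds the NSLaser Niagara "Beam End" variable, so the beam stops at obstacles.
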(event EventBeginPlay)

(event Collision|EventActorBeginOverlap
  (params (OtherActor :type Actor%20Object%20Reference)))

(event EventTick
  (params (DeltaSeconds :type Float%20%28single-precision%29))
  (bind _sphere (Variables|Default|GetSphere))
  (bind _returnvalue (Transformation|GetWorldLocation _sphere))
  (Transformation|AddWorldRotation _sphere (Math|Rotator|MakeRotator 0.0 0.0 (* DeltaSeconds (Variables|Default|GetRotationSpeed))) false false)
  (bind _outhit (Collision|LineTraceByChannel _returnvalue (+ _returnvalue (* (Math|Vector|GetForwardVector _sphere) 1e+04)) "TraceTypeQuery1" false 0 "None"))
  (Class|NiagaraComponent|SetNiagaraVariableVec3 (Variables|Default|GetNS_Laser) "Beam End" (Math|Vector|SelectVector (.ImpactPoint (Collision|BreakHitResult _outhit)) (.TraceEnd (Collision|BreakHitResult _outhit)) (.bBlockingHit (Collision|BreakHitResult _outhit)))))

(fn ConstructionScript)